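; BP_Crosses is a proximity effect actor that animates the yaw of its static mesh when the effect starts and ends.
; EffectStart plays one timeline to drive the rotation, then plays a second one on finish if nothing is still overlapping.
; EndEffect plays that second timeline only when the first is not running, so the opening rotation always completes before the closing one begins.
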(event `self.ReceiveTick`
  (params (DeltaSeconds :type "Float (single-precision)"))
  (`parent.ReceiveTick` DeltaSeconds))

(event `self.EffectStart`
  (bind _staticmesh (`self.StaticMesh`))
  (bind _staticmesh_2 (`self.StaticMesh`))
  (bind (_relativerotation_roll _relativerotation_pitch) (`KismetMathLibrary.BreakRotator` (`SceneComponent.RelativeRotation` _staticmesh)))
  (bind (_relativerotation_roll_2 _relativerotation_pitch_2) (`KismetMathLibrary.BreakRotator` (`SceneComponent.RelativeRotation` _staticmesh_2)))
  (bind (_direction _newtrack_0) (`Timeline|Timeline_0` :!via `PlayFromStart`)
    (:`Update`
      (`SceneComponent.K2_SetRelativeRotation` _staticmesh_2 (`KismetMathLibrary.MakeRotator` _relativerotation_roll_2 _relativerotation_pitch_2 _newtrack_0) false false))
    (:`Finished`
      (if (not (`self.IsOverlapping`))
        (bind (_direction_2 _newtrack_0_2) (`Timeline|Timeline_1` :!via `PlayFromStart` :!label _label)
          (:`Update`
            (`SceneComponent.K2_SetRelativeRotation` _staticmesh (`KismetMathLibrary.MakeRotator` _relativerotation_roll _relativerotation_pitch _newtrack_0_2) false false)))))))

(event `self.EndEffect`
  (if (not (`TimelineComponent.IsPlaying` (`self.Timeline_0`)))
    (goto _label :!via `PlayFromStart`)))

(fn `UserConstructionScript`
  (`parent.UserConstructionScript`))