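; BP_ProximityEffect is a base proximity trigger with empty EffectStart and EffectEnd events, apparently meant for child Blueprints to fill.
; Sphere overlap starts the effect for one WIWCharacter that is not locally controlled, and ends it when that actor leaves.
; IsOverlapping is set before the cast and control check, so a rejected first actor blocks later starts.
; Both overlap events print the actor's name for debugging.
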(event `self.Sphere.OnComponentBeginOverlap`
  (params (OverlappedComponent :type "PrimitiveComponent Object Reference") (OtherActor :type "Actor Object Reference") (OtherComp :type "PrimitiveComponent Object Reference") (OtherBodyIndex :type Integer) (bFromSweep :type Boolean) (SweepResult :type "HitResult Structure (by ref)"))
  (`KismetSystemLibrary.PrintString` (`KismetSystemLibrary.GetDisplayName` OtherActor))
  (if (not (`self.IsOverlapping`))
    (set `self.IsOverlapping` true)
    (bind _aswiwcharacter (cast `WIWCharacter` OtherActor))
    (if (not (`Pawn.IsLocallyControlled` _aswiwcharacter))
      (set `self.OverlappingActor` _aswiwcharacter)
      (`self.EffectStart`))))

(event `self.Sphere.OnComponentEndOverlap`
  (params (OverlappedComponent :type "PrimitiveComponent Object Reference") (OtherActor :type "Actor Object Reference") (OtherComp :type "PrimitiveComponent Object Reference") (OtherBodyIndex :type Integer))
  (`KismetSystemLibrary.PrintString` (`KismetSystemLibrary.GetDisplayName` OtherActor))
  (if (== OtherActor (`self.OverlappingActor`))
    (`self.EffectEnd`)
    (set `self.IsOverlapping` false)
    (set `self.OverlappingActor` null)))

(event `EffectStart`)

(event `EffectEnd`)

(fn `UserConstructionScript`)