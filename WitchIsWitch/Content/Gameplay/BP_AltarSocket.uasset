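; BP_AltarSocket is an interactable socket on an altar where a held item is placed.
; On Interact, it makes the interactor drop its HeldItem, then moves that item to the ItemLocator transform.
; It then asks its linked Altar to run CheckRecipe, so recipe evaluation lives in the altar rather than the socket.
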(event `self.Interact`
  (params (interactor :type "WIWCharacter Object Reference"))
  (bind _helditem (`WIWCharacter.HeldItem` interactor))
  (bind _altar (`self.Altar`))
  (`/Engine/EditorBlueprintResources/StandardMacros.IsValid` interactor
    (:`Is Valid`
      (`/Engine/EditorBlueprintResources/StandardMacros.IsValid` _helditem
        (:`Is Valid`
          (bind _output_get (set `self.Item` _helditem))
          (`WIWPickupable.Drop` _helditem)
          (`self.K2_SetActorTransform` _output_get (`SceneComponent.K2_GetComponentToWorld` (`self.ItemLocator`)) false false)
          (`/Engine/EditorBlueprintResources/StandardMacros.IsValid` _altar
            (:`Is Valid`
              (`/Game/Gameplay/BP_Altar.CheckRecipe` _altar))))))))

(fn `UserConstructionScript`)