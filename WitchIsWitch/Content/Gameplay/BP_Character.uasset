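; First-person multiplayer player character with a timed hunt mode that fades the goat material on bodies.
; Z starts a hunt locally and relays it via server multicast, changing walk speed and camera FOV until Tick times it out.
; UpdateVisibility targets full Fade while any character hunts, interpolated each Tick.
; Kill shows the local victim a death animation through another actor and ends hunts, while Reset clears state and rotates non-weapon item spawns.
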(event `Kill`
  (params (Instigator :type "/Game/Gameplay/BP_Character Object Reference"))
  (if (`self.IsLocallyControlled`)
    (bind _outactors (`GameplayStatics.GetAllActorsOfClass` "/Game/NewBlueprint.NewBlueprint_C"))
    (bind _output (`|GetArrayItem` _outactors))
    (bind _skeletalmesh (`/Game/NewBlueprint.SkeletalMesh` _output))
    (`SceneComponent.SetVisibility` _skeletalmesh true false)
    (`SceneComponent.K2_SetWorldTransform` (`/Game/NewBlueprint.DefaultSceneRoot` _output) (`SceneComponent.K2_GetComponentToWorld` (`Character.Mesh` Instigator)) false false)
    (`PlayerController.SetViewTargetWithBlend` (`GameplayStatics.GetPlayerController` 0) _output 0.0 "VTBlend_Linear" 0.0 false)
    (`SkeletalMeshComponent.Play` _skeletalmesh false)
    (bind _outactors_2 (`GameplayStatics.GetAllActorsOfClass` "BP_Character_C"))
    (for _array_element _outactors_2
      (set `/Game/Gameplay/BP_Character.bIsInHuntMode` false _array_element))
    (for _array_element_2 _outactors_2
      (set `/Game/Gameplay/BP_Character.InstantFade` true _array_element_2)
      (`self.Update Visibility` _array_element_2))
    (`KismetSystemLibrary.Delay` 2.3)
    (`KismetSystemLibrary.PrintString` "Reset")))

(event `self.ReceiveBeginPlay`
  (`KismetSystemLibrary.K2_SetTimerDelegate` (delegate `CustomEvent_0`) 2.0 true)
  (set `CharacterMovementComponent.MaxWalkSpeed` (`self.WalkSpeed`) (`self.CharacterMovement`))
  (bind _returnvalue (`|CreateWidget` "/Game/UI/WBP_Overlay.WBP_Overlay_C" (`GameplayStatics.GetPlayerController` 0)))
  (`UserWidget.AddToViewport` _returnvalue 0)
  (set `self.NewVar_0` _returnvalue)
  (`SceneComponent.SetVisibility` (`self.Mesh`) (not (`self.IsLocallyControlled`)) false)
  (`self.Update Visibility`))

(event `CustomEvent_0`
  (`self.Update Visibility`))

(event `self.ReceiveTick`
  (params (DeltaSeconds :type "Float (single-precision)"))
  (bind _output_get (set `self.CurrentVisibility` (`KismetMathLibrary.SelectFloat` (`self.TargetVisibility`) (`KismetMathLibrary.FInterpTo` (`self.CurrentVisibility`) (`self.TargetVisibility`) DeltaSeconds 1.0) (`self.InstantFade`))))
  (`MaterialInstanceDynamic.SetScalarParameterValue` (`self.Material`) "Fade" _output_get)
  (`WIWOverlay.JankyTick` (`self.NewVar_0`))
  (if (`self.bIsInHuntMode`)
    (set `self.HuntModeTimer` (+ (`self.HuntModeTimer`) DeltaSeconds))
    (if (> (`self.HuntModeTimer`) (`self.HuntModeDuration`))
      (`self.EndHunt`))))

(event `InputAxis|MoveForward`
  (params (AxisValue :type "Float (single-precision)"))
  ;[1 1 1] Camera, movement
  (`self.AddMovementInput` (`SceneComponent.GetForwardVector` (`self.Camera`)) AxisValue))

(event `InputAxis|LookUp`
  (params (AxisValue :type "Float (single-precision)"))
  ;[1 1 1] Camera, movement
  (`self.AddControllerPitchInput` AxisValue))

(event `InputAxis|MoveRight`
  (params (AxisValue :type "Float (single-precision)"))
  ;[1 1 1] Camera, movement
  (`self.AddMovementInput` (`SceneComponent.GetRightVector` (`self.Camera`)) AxisValue))

(event `InputAxis|LookSideways`
  (params (AxisValue :type "Float (single-precision)"))
  ;[1 1 1] Camera, movement
  (`self.AddControllerYawInput` AxisValue))

(event `Key|Z`
  (params (Key :type "Key Structure"))
  (:`Pressed`
    (`self.Local_Hunt`)
    (`self.Server_Hunt` (`self.GetPlayerID`))))

(event `Server_Hunt`
  (params (PlayerID :type Integer))
  (`self.Multicast_Hunt` PlayerID))

(event `Multicast_Hunt`
  (params (PlayerID :type Integer))
  (if (!= PlayerID (`self.GetPlayerID`))
    (`self.Local_Hunt`)))

(event `EndHunt`
  (if (`self.bIsInHuntMode`)
    ;[1 1 1] Camera FOV change & Timer
    (set `CharacterMovementComponent.MaxWalkSpeed` (`self.WalkSpeed`) (`self.CharacterMovement`) :!label _label)
    (if (`self.bIsInHuntMode`)
      (bind _outactors (`GameplayStatics.GetAllActorsOfClass` "BP_Character_C"))
      (for _array_element _outactors
        (bind _asbp_character (cast `/Game/Gameplay/BP_Character` _array_element))
        (`self.Update Visibility` _asbp_character))
      (set `self.bIsInHuntMode` false)
      (bind (_direction _fov) (`Timeline|CameraFOV` :!via `ReverseFromEnd` :!label _label_2)
        (:`Update`
          (`CameraComponent.SetFieldOfView` (`self.Camera`) _fov))
        (:`Finished`
          (if (`self.bIsInHuntMode`)
            (`KismetSystemLibrary.Delay` (- (`self.HuntModeDuration`) (`TimelineComponent.GetTimelineLength` (`self.CameraFOV`))))
            (goto _label)))))))

(event `Local_Hunt`
  ;[1 1 1] Begin Hunt
  (if (not (`self.bIsInHuntMode`))
    (set `CharacterMovementComponent.MaxWalkSpeed` (`self.HuntWalkSpeed`) (`self.CharacterMovement`))
    (set `self.HuntModeTimer` 0.0)
    (set `self.bIsInHuntMode` true)
    (`KismetSystemLibrary.PrintString` "Pick up knife etc")
    (bind _outactors (`GameplayStatics.GetAllActorsOfClass` "BP_Character_C"))
    (for _array_element _outactors
      (bind _asbp_character (cast `/Game/Gameplay/BP_Character` _array_element))
      (`self.Update Visibility` _asbp_character))
    (goto _label_2 :!via `PlayFromStart`)))

(fn `Reset`
  (bind _itemspawnlocationarray (`self.ItemSpawnLocationArray`))
  (bind _outactors (`GameplayStatics.GetAllActorsOfClass` "/Script/WitchIsWitch.WIWItem"))
  (for _array_element _outactors
    (cast `/Game/Gameplay/Items/BP_Item_Weapon` _array_element
      (:`CastFailed`
        (bind _returnvalue (`KismetArrayLibrary.Array_Add` (`self.ItemSpawnLocationArray`) (`WIWItem.InitialTransform` _array_element)))
        (`BlueprintMapLibrary.Map_Add` (`self.Spawn Position Dict`) _array_element _returnvalue))))
  (set `self.bIsInHuntMode` false)
  (set `self.CurrentVisibility` 0.0)
  (set `self.TargetVisibility` 0.0)
  (set `self.HuntModeTimer` 0.0)
  (set `CharacterMovementComponent.MaxWalkSpeed` (`self.WalkSpeed`) (`self.CharacterMovement`))
  (bind _outactors_2 (`GameplayStatics.GetAllActorsOfClass` "/Script/WitchIsWitch.WIWItem"))
  (for _array_element_2 _outactors_2
    (bind (_value _returnvalue_2) (`BlueprintMapLibrary.Map_Find` (`self.Spawn Position Dict`) _array_element_2))
    (if _returnvalue_2
      (set `WIWItem.InitialTransform` (`|GetArrayItem` _itemspawnlocationarray (mod (+ _value 1) (`KismetArrayLibrary.Array_Length` _itemspawnlocationarray))) _array_element_2)
      (`WIWPickupable.Reset` _array_element_2))))

(fn `Update Visibility`
  (bind _outactors (`GameplayStatics.GetAllActorsOfClass` "BP_Character_C"))
  (for _array_element _outactors
    (bind _asbp_character (cast `/Game/Gameplay/BP_Character` _array_element)
      (:`then`
        (if (`/Game/Gameplay/BP_Character.bIsInHuntMode` _asbp_character)
          (set `self.TargetVisibility` 1.0)
          (return)))
      (:`CastFailed`
        (return))))
  (set `self.TargetVisibility` 0.0)
  (return))

(fn `UserConstructionScript`
  (bind _returnvalue (`PrimitiveComponent.CreateDynamicMaterialInstance` (`self.Mesh`) 0 "/Game/Characters/Goat/M_Goat.M_Goat" "None"))
  (bind _output_get (set `self.Material` _returnvalue))
  (`PrimitiveComponent.SetMaterial` (`self.Mesh`) 0 _output_get))