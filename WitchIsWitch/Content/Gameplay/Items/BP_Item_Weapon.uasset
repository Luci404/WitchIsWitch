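; Weapon item Blueprint that instantly kills the character it hits when used.
; On Use, it casts the interactor to BP_Character and line traces from that character's camera along its forward vector for Range, ignoring the user.
; A blocking hit on another BP_Character calls Kill with the user as argument and prints a debug string.
; The trace is a single hitscan check, with no damage amount, ammo or effects.
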(event `self.Use`
  (bind _returnvalue (`self.GetInteractor` self))
  (bind _asbp_character (cast `/Game/Gameplay/BP_Character` _returnvalue))
  (bind _camera (`/Game/Gameplay/BP_Character.Camera` _asbp_character))
  (bind _returnvalue_2 (`SceneComponent.K2_GetComponentLocation` _camera))
  (bind _outhit (`KismetSystemLibrary.LineTraceSingle` _returnvalue_2 (+ _returnvalue_2 (* (`SceneComponent.GetForwardVector` _camera) (`self.Range`))) "TraceTypeQuery4" false (`|MakeArray` _asbp_character :!type "Actor Object Reference")))
  (bind (_bblockinghit _binitialoverlap _time _distance _location _impactpoint _normal _impactnormal _physmat _hitactor) (`GameplayStatics.BreakHitResult` _outhit))
  (if _bblockinghit
    (bind _asbp_character_2 (cast `/Game/Gameplay/BP_Character` _hitactor))
    (`/Game/Gameplay/BP_Character.Kill` _asbp_character_2 _asbp_character)
    (`KismetSystemLibrary.PrintString` "try kill")))

(fn `UserConstructionScript`)