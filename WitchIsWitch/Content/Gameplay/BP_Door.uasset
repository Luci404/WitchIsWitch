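; BP_Door is an interactable door that swings open and closed around its yaw in a configurable direction.
; BeginPlay caches the starting rotation and, based on OpenClockwise, tags one of the two direction-specific blocking volumes "InteractBlock".
; Each Interact from a valid interactor alternates via FlipFlop between playing and reversing the OpenDoor timeline.
; The timeline's yaw curve offsets the Scene component's world rotation from the cached rotation.
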(event `self.ReceiveBeginPlay`
  (set `self.OriginalRotation` (`self.K2_GetActorRotation`))
  (set `ActorComponent.ComponentTags` (`|MakeArray` "InteractBlock" :!type "Name") (select `bool` (`self.bOpenClockwise`) :`false` (`self.Clockwise_BlockingVolume`) :`true` (`self.CounterClockwose_BlockingVolume`))))

(event `self.Interact`
  (params (interactor :type "WIWCharacter Object Reference"))
  (bind (_originalrotation_roll _originalrotation_pitch _originalrotation_yaw) (`KismetMathLibrary.BreakRotator` (`self.OriginalRotation`)))
  (`/Engine/EditorBlueprintResources/StandardMacros.IsValid` interactor
    (:`Is Valid`
      (`/Engine/EditorBlueprintResources/StandardMacros.FlipFlop`
        (:`A`
          (bind (_direction _yaw) (`Timeline|OpenDoor` :!label _label)
            (:`Update`
              (`SceneComponent.K2_SetWorldRotation` (`self.Scene`) (`KismetMathLibrary.MakeRotator` _originalrotation_roll _originalrotation_pitch (`KismetMathLibrary.SelectFloat` (+ _originalrotation_yaw _yaw) (- _originalrotation_yaw _yaw) (`self.bOpenClockwise`))) false false))))
        (:`B`
          (goto _label :!via `Reverse`))))))

(fn `UserConstructionScript`)